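; Enemy actor that supports player lock-on by showing a skull marker and exposing targeting data.
; The Lockon event flip-flops the skull's visibility, and Tick rotates the visible skull toward the player character.
; DistanceToPlayer line-traces pawn objects toward the player with debug drawing, stores the hit distance and flags the enemy as targetable regardless of the result.
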(event `/Game/Blueprints/Enemies/EnemyLockOn.LockOn`
  (`/Engine/EditorBlueprintResources/StandardMacros.FlipFlop`
    (:`A`
      (`SceneComponent.SetVisibility` (`self.Skull`) true false)
      (set `self.SkullVisible` true))
    (:`B`
      (`SceneComponent.SetVisibility` (`self.Skull`) false false)
      (set `self.SkullVisible` false))))

(event `self.ReceiveTick`
  (params (DeltaSeconds :type "Float (single-precision)"))
  (`KismetSystemLibrary.Delay` 0.01)
  (if (`self.SkullVisible`)
    (cast `/Game/Blueprints/Character/ThirdPersonCharacter` (`GameplayStatics.GetPlayerCharacter` 0))
    (`SceneComponent.K2_SetWorldRotation` (`self.Skull`) (`KismetMathLibrary.FindLookAtRotation` (`self.K2_GetActorLocation`) (`self.K2_GetActorLocation` (`GameplayStatics.GetPlayerCharacter` 0))) false false)))

(fn `DistanceToPlayer`
  (bind _outhit (`KismetSystemLibrary.LineTraceSingleForObjects` (`self.K2_GetActorLocation`) (`self.K2_GetActorLocation` (`GameplayStatics.GetPlayerPawn` 0)) (`|MakeArray` "ObjectTypeQuery3" :!type "EObjectTypeQuery Enum") false (`|MakeArray` self :!type "Actor Object Reference") "ForDuration" true (struct :`R` 1.0 :`A` 1.0) (struct :`G` 1.0 :`A` 1.0) 0.1))
  (set `self.PlayertoEnemyDistance` (`.Distance` (`GameplayStatics.BreakHitResult` _outhit)))
  (set `self.CanBeTargeted?` true)
  (return))

(fn `UserConstructionScript`)